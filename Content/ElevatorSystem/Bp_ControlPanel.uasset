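; Elevator control panel that builds a grid of floor buttons at runtime, one per floor.
; On BeginPlay it lays out mesh components from a start transform, wrapping into a new row below whenever the horizontal limit is reached.
; Each button is tagged as an elevator button with its zero-based floor index and gets a one-based text label.
; The same loop tells the linked elevator's call button object to spawn a button for each floor.
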(event EventBeginPlay
  (Variables|Default|SetControl%20Panel%20Button%20OffsetCache (Variables|ControlPanelButton|GetControlPanelButtonOffset))
  (Variables|Default|SetMax%20Horizontal%20ButtonCache (Variables|ControlPanelButton|GetMaxHorizontalButton))
  (Variables|Default|SetStart%20Transform (Transformation|GetRelativeTransform (Variables|Default|GetStartPosition)))
  (for _index (range 1 (Variables|Default|GetNumber%20of%20Floors))
    (Variables|Default|SetCurrentLine%20Value _index)
    (if (> (Variables|Default|GetCurrentLine%20Value) (Variables|ControlPanelButton|GetMaxHorizontalButton))
      (Variables|Default|SetNewLineValue%20 (+ (Variables|Default|GetNewLineValue%20) (Variables|Default|GetControlPanelButtonDistanceBetweenVertical)))
      (Variables|ControlPanelButton|SetControlPanelButtonOffset (Variables|Default|GetControl%20Panel%20Button%20OffsetCache))
      (Variables|ControlPanelButton|SetMaxHorizontalButton (+ (Variables|ControlPanelButton|GetMaxHorizontalButton) (Variables|Default|GetMax%20Horizontal%20ButtonCache))))
    (bind _returnvalue (AddComponent|AddStaticMeshComponent false (Variables|Default|GetStart%20Transform)))
    (bind _output_get (Variables|Default|SetButtonMeshCompRef _returnvalue))
    (Variables|/Script/Engine.ActorComponent|SetComponentTags _output_get (Utilities|Array|MakeArray "ElevatorButton" (Utilities|String|StringToName (Utilities|String|ToString(Integer) (- (Variables|Default|GetCurrentLine%20Value) 1)))))
    (Transformation|SetRelativeLocation (Variables|Default|GetButtonMeshCompRef) (Math|Vector|MakeVector (.x (.location (Variables|Default|GetStart%20Transform))) (- (Variables|ControlPanelButton|GetControlPanelButtonOffset) (.y (.location (Variables|Default|GetStart%20Transform)))) (- (.z (.location (Variables|Default|GetStart%20Transform))) (Variables|Default|GetNewLineValue%20))) false false)
    (Variables|ControlPanelButton|SetControlPanelButtonOffset (- (Variables|ControlPanelButton|GetControlPanelButtonOffset) (Variables|Default|GetControlPanelButtonDistanceBetweenHorizontal)))
    (Default|SpawnButton (Variables|/Game/ElevatorSystem/BP_Elevator.BP_Elevator_C|GetElevatorCallButtonRef (Variables|Default|GetElevatorRef)) (Utilities|String|StringToName (Utilities|String|ToString(Integer) (- (Variables|Default|GetCurrentLine%20Value) 1))))
    (bind _returnvalue_2 (AddComponent|AddTextRenderComponent false (Math|Transform|MakeTransform (Math|Vector|MakeVector (.x (Variables|/Script/Engine.SceneComponent|GetRelativeLocation (Variables|Default|GetButtonMeshCompRef))) (.y (Variables|/Script/Engine.SceneComponent|GetRelativeLocation (Variables|Default|GetButtonMeshCompRef))) (.z (Variables|/Script/Engine.SceneComponent|GetRelativeLocation (Variables|Default|GetButtonMeshCompRef)))) "0, 0, 0" "1.000000,1.000000,1.000000")))
    (Rendering|Components|TextRender|SetText _returnvalue_2 (Utilities|Text|ToText(Integer) (+ (Math|Conversions|ToInteger(Byte) (Utilities|String|ToString(Text) (Utilities|Text|ToText(Name) (Utilities|String|StringToName (Utilities|String|ToString(Integer) (- (Variables|Default|GetCurrentLine%20Value) 1)))))) 1)))))

(fn ConstructionScript)