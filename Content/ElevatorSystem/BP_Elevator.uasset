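; Elevator actor that spawns its own call button and control panel, passing each its layout settings and a back-reference.
; The panel is attached to the elevator.
; Floor requests print a debug message and run a timeline that scales one door on X.
; It looks unfinished: no cabin movement exists, the busy flag is never set true, and the door's Open input is ignored, so reverse playback never runs.
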(event Custom|GoToFloorEvent
  (params (Floor :type Integer))
  (if (not (Variables|Default|GetCurrentlyActive?))
    (Variables|Default|SetFloor%20toRef Floor)
    (if (== (Variables|Default|GetFloor%20toRef) (Variables|Default|GetWhatFloorWeAt?))
      (Development|PrintString (Utilities|String|Append "Already at floor:" (Utilities|String|ToString(Integer) (Variables|Default|GetFloor%20toRef)) "" "Oppening Doors"))
      (CallFunction|OpenCloseElevatorDoor false)
      (else
        (Variables|Default|SetCurrentlyActive? false)
        (Development|PrintString (Utilities|String|Append "Going to floor" (Utilities|String|ToString(Integer) (Variables|Default|GetFloor%20toRef)) "" "Closing the doors"))
        (CallFunction|OpenCloseElevatorDoor false)))))

(event Custom|OpenCloseElevatorDoor
  (params (Open? :type Boolean))
  (Components|Timeline|SetPlayRate (Variables|Default|GetOpenCloseElevatorDoorTimeLine) (/ 1.0 (Variables|Default|GetElevatorDoorSpeed)))
  (if true
    (bind _opencloseelevatordoorfloattrack (Timeline|OpenCloseElevatorDoorTimeLine PlayFromStart)
      (:Update
        (Transformation|SetRelativeScale3D (Variables|Default|GetDoor1) (Math|Vector|MakeVector (Math|Float|Lerp 1.5 0.1 _opencloseelevatordoorfloattrack) 0.0 0.0))))
    (else
      (Timeline|OpenCloseElevatorDoorTimeLine ReverseFromEnd))))

(event EventBeginPlay
  (bind _controlpanelarrow (Variables|Default|GetControlPanelArrow))
  (bind _returnvalue (Transformation|GetWorldLocation _controlpanelarrow))
  (bind _returnvalue_2 (Game|SpawnActorfromClass "/Game/ElevatorSystem/BP_ElevatorCallButton.BP_ElevatorCallButton_C" (Math|Transform|MakeTransform (.location (Transformation|GetWorldTransform (Variables|Default|GetButtonArrow))) "0, 0, 0" "1.000000,1.000000,1.000000") "Undefined" "MultiplyWithRoot" 0 (Variables|CallButton|GetCall%20Button%20Vert%20Offset) (Variables|CallButton|GetCall%20Button%20Hor%20Offset) (Variables|CallButton|GetCall%20Button%20Depth%20Offset) (Variables|CallButton|GetCall%20Button%20Mesh) self 0))
  (Variables|Default|SetElevatorCallButtonRef _returnvalue_2)
  (bind _returnvalue_3 (Game|SpawnActorfromClass "/Game/ElevatorSystem/Bp_ControlPanel.Bp_ControlPanel_C" (Math|Transform|MakeTransform (Math|Vector|MakeVector (+ (.x _returnvalue) (Variables|CallButton|GetCall%20Button%20Depth%20Offset)) (+ (.y _returnvalue) (Variables|ControlPanelPanel|GetControlPanelHorizontalOffset)) (+ (.z _returnvalue) (Variables|ControlPanelPanel|GetControlPanelVertOffset))) "0, 0, 0" "1.000000,1.000000,1.000000") "Undefined" "MultiplyWithRoot" 0 (Variables|ElevatorControlPanel|GetControl%20Panel%20Button%20Offset) (Variables|ElevatorControlPanel|GetMax%20Horizontal%20Button) (Variables|Floors|GetNumber%20Of%20Floors) (Variables|ElevatorControlPanel|GetControl%20Panel%20Button%20Distance%20Between%20Horizontal) (Variables|ElevatorControlPanel|GetControl%20Panel%20Button%20Distance%20Between%20Vertical) self 0))
  (Transformation|AttachActorToActor _returnvalue_3 self "None" "KeepWorld" "KeepWorld" "KeepWorld" true))

(fn ConstructionScript)